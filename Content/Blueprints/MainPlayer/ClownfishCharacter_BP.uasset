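; Player clownfish character Blueprint that detects when it is close enough to a fish to interact with it.
; Begin and end overlap events store the other actor in CollidedActor and, if it has the "Fish" tag, set or clear the CanInteract flag.
; The flag is a simple boolean with no overlap count, and this graph does not act on it.
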(event `self.ReceiveBeginPlay`)

(event `self.ReceiveTick`
  (params (DeltaSeconds :type "Float (single-precision)")))

(event `self.ReceiveActorBeginOverlap`
  (params (OtherActor :type "Actor Object Reference"))
  (bind _output_get (set `self.collidedActor` OtherActor))
  (if (`self.ActorHasTag` _output_get "Fish")
    (set `self.canInteract` true)))

(event `self.ReceiveActorEndOverlap`
  (params (OtherActor :type "Actor Object Reference"))
  (bind _output_get (set `self.collidedActor` OtherActor))
  (if (`self.ActorHasTag` _output_get "Fish")
    (set `self.canInteract` false)))

(fn `UserConstructionScript`)