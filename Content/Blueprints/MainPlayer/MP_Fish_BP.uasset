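; Main player Blueprint that sets up the HUD and tracks when the player can interact with fish.
; On BeginPlay it creates and shows the OLD_HUD widget and hides the mouse cursor.
; Every Tick it converts the crosshair image's geometry into a viewport pixel position and stores it.
; Actor overlaps with anything tagged "Fish" toggle the CanInteract flag, though nothing in this graph reads that flag or the crosshair position.
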(event `self.ReceiveBeginPlay`
  (bind _returnvalue (`GameplayStatics.GetPlayerController` 0))
  (bind _returnvalue_2 (`|CreateWidget` "/Game/Blueprints/UI/OLD_HUD.OLD_HUD_C" _returnvalue))
  (`UserWidget.AddToViewport` _returnvalue_2 0)
  (set `PlayerController.bShowMouseCursor` false _returnvalue))

(event `self.ReceiveTick`
  (params (DeltaSeconds :type "Float (single-precision)"))
  (set `self.crossHairScreenLoc` (`SlateBlueprintLibrary.LocalToViewport` (`Widget.GetTickSpaceGeometry` (`/Game/Blueprints/UI/OLD_HUD.CrossHair_Img` (stale `self.ReceiveBeginPlay` _returnvalue_2))))))

(event `self.ReceiveActorBeginOverlap`
  (params (OtherActor :type "Actor Object Reference"))
  (bind _output_get (set `self.collidedActor` OtherActor))
  (if (`self.ActorHasTag` _output_get "Fish")
    (set `self.canInteract` true)))

(event `self.ReceiveActorEndOverlap`
  (params (OtherActor :type "Actor Object Reference"))
  (bind _output_get (set `self.collidedActor` OtherActor))
  (if (`self.ActorHasTag` _output_get "Fish")
    (set `self.canInteract` false)))

(fn `UserConstructionScript`)